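; Actor component that bridges Reaper and Unreal, playing Reaper's output at the owning actor through audio capture.
; It spawns and attaches a BP_AudioCapture, replacing any found instance, and expects Reaper routed into the microphone input.
; Sound settings are set manually or copied from audio components or sound assets, whose original volumes are cached and restored on EndPlay.
; OSC helpers trigger Reaper actions like stop and play from edit cursor.
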(event EventBeginPlay)

(event EventTick
  (params (DeltaSeconds :type Float%20%28single-precision%29)))

(event EventEndPlay
  (params (EndPlayReason :type EEndPlayReason%20Enum :default "Destroyed"))
  (switch Utilities|FlowControl|Switch|SwitchonEEndPlayReason EndPlayReason
    (:Destroyed
      _)
    (:LevelTransition
      _)
    (:EndPlayInEditor
      _)
    (:RemovedFromWorld
      _)
    (:Quit
      _))
  (CallFunction|RestoreSoundSettings))

(fn PlaceAudiofromReaper
  (bind _returnvalue (Actor|GetActorOfClass "/ReaperUnrealBridge/BP_AudioCapture.BP_AudioCapture_C"))
  (if (Utilities|IsValid _returnvalue)
    (Actor|DestroyActor _returnvalue)
    (CallFunction|SpawnActor)
    (Default|StartAudioCapture (Variables|Components|GetSpawned%20Actor))
    (CallFunction|AttachActortoActor)
    (else
      (CallFunction|SpawnActor)
      (Default|StartAudioCapture (Variables|Components|GetSpawned%20Actor))
      (CallFunction|AttachActortoActor))))

(fn SpawnActor
  ;[0.15 0.15 0.15 0.5] Spawn a Blueprint Actor that contains the Audio Capture component. That component gets audio from your microphone input, which should be routed to be a digital output from Reaper in other for the plugin to work
  (bind _returnvalue (Game|SpawnActorfromClass "/ReaperUnrealBridge/BP_AudioCapture.BP_AudioCapture_C" (Math|Transform|MakeTransform "0, 0, 0") "AlwaysSpawn" "MultiplyWithRoot" (Components|GetOwner) 0))
  (Variables|Components|SetSpawned%20Actor _returnvalue))

(fn AttachActortoActor
  ;[0.15 0.15 0.15 0.5] Attached the AudioCapture with Debug Sphere to the actor that containts this component
  (Transformation|AttachActorToActor (Variables|Components|GetSpawned%20Actor) (Components|GetOwner) "None" "KeepRelative" "KeepRelative" "KeepRelative" true))

(fn StartStream
  (Default|StartAudioCapture (Variables|Components|GetSpawned%20Actor)))

(fn StopStream
  (Default|StopAudioCapture (Variables|Components|GetSpawned%20Actor)))

(fn SetSoundSettings
  (params (SoundClass :type Sound%20Class%20Object%20Reference) (Attenuation%20Settings :type Sound%20Attenuation%20Object%20Reference) (AdjustVolumeLevel :type Float%20%28single-precision%29))
  (bind _spawned_actor (Variables|Components|GetSpawned%20Actor))
  (bind _audiocaptureinbp (Variables|/ReaperUnrealBridge/BP_AudioCapture.BP_AudioCapture_C|GetAudioCaptureInBP _spawned_actor))
  ;[0.15 0.15 0.15 0.5] Manually set sound class, attenuation and volume on your AudioCapture
  (Class|ReaperAudioHelpers|SetAttenuationonSynthComponent _audiocaptureinbp Attenuation%20Settings)
  (Class|ReaperAudioHelpers|SetSoundClassonSynthComponent _audiocaptureinbp SoundClass)
  (Audio|Components|Audio|AdjustVolume _audiocaptureinbp 0.0 AdjustVolumeLevel "Linear" :!class /Script/AudioMixer.SynthComponent))

(fn OSCSend
  ;[0.15 0.15 0.15 0.5] Sends OSC to Reaper. Double check that the IP adress and Port matches your settings in Reaper
  (Class|ReaperOSCSender|QuickSendMessage (Variables|Settings|GetOSC%20Ip%20Adress) (Variables|Settings|GetOSC%20Port) (Variables|Default|GetOSC%20Message) 1.0))

(fn OSCSendStop
  (Variables|Default|SetOSC%20Message (Utilities|String|Append "/action/" (|GetReaperAction)))
  (CallFunction|OSCSend))

(fn OSCSendPlayfromEditCursor
  (Variables|Default|SetOSC%20Message (Utilities|String|Append "/action/" (|GetReaperAction)))
  (CallFunction|OSCSend))

(fn OSCSendAction
  (params (Action%20ID :type String))
  ;[0.15 0.15 0.15 0.5] This function is hard coded to trigger an Action, but you can modify it to other OSC messsages as well
  (Variables|Default|SetOSC%20Message (Utilities|String|Append "/action/" Action%20ID))
  (CallFunction|OSCSend))

(fn DebugSounds
  (params (bPrintToScreen :type Boolean))
  (Class|ReaperAudioHelpers|DebugLogAudioSettings (Variables|/ReaperUnrealBridge/BP_AudioCapture.BP_AudioCapture_C|GetAudioCaptureInBP (Variables|Components|GetSpawned%20Actor)) bPrintToScreen))

(fn CopySettingsfromAudioComponent
  (params (SourceComponent :type Audio%20Component%20Object%20Reference) (bMuteSource :type Boolean))
  ;[0.15 0.15 0.15 0.5] Stores all Audio Component in a map,  skips add if the Audio Component is already added.
  (bind _output_get (Variables|SourceAudio|SetSource%20Component SourceComponent))
  (CallFunction|StopStream)
  (bind _originalvolumemultiplier (Class|ReaperAudioHelpers|CopySettingsfromAudioComponent (Variables|/ReaperUnrealBridge/BP_AudioCapture.BP_AudioCapture_C|GetAudioCaptureInBP (Variables|Components|GetSpawned%20Actor)) (Variables|SourceAudio|GetSource%20Component) bMuteSource))
  (if (Utilities|Map|Contains (Variables|SourceAudio|GetAudiComponentMap) _output_get)
    _
    (else
      (Utilities|Map|Add (Variables|SourceAudio|GetAudiComponentMap) (Variables|SourceAudio|GetSource%20Component) _originalvolumemultiplier)))
  (CallFunction|StartStream))

(fn CopySettingsfromSoundBase
  (params (SoundAsset :type Sound%20Base%20Object%20Reference) (bMuteSource :type Boolean))
  ;[0.15 0.15 0.15 0.5] Stores all sound bases in a map,  skips add if the sound base is already added.
  (LocalVariables|SetSoundBase SoundAsset)
  (CallFunction|StopStream)
  (bind _originalvolume (Class|ReaperAudioHelpers|CopySettingsfromSoundBase (Variables|/ReaperUnrealBridge/BP_AudioCapture.BP_AudioCapture_C|GetAudioCaptureInBP (Variables|Components|GetSpawned%20Actor)) (LocalVariables|GetSoundBase) bMuteSource))
  (if (Utilities|Map|Contains (Variables|SourceAudio|GetSoundBaseMap) SoundAsset)
    _
    (else
      (Utilities|Map|Add (Variables|SourceAudio|GetSoundBaseMap) (LocalVariables|GetSoundBase) _originalvolume)))
  (CallFunction|StartStream))

(fn RestoreSoundSettings
  ;[0.15 0.15 0.15 0.5] Restore Volume to Audio Components
  (bind (_keypin _valuepin) (Utilities|Map|ForEachLoop(Map) (Variables|SourceAudio|GetAudiComponentMap))
    (:then
      (Class|ReaperAudioHelpers|RestoreVolumeMultiplier _keypin _valuepin))
    (:CompletedPin
      ;[0.15 0.15 0.15 0.5] Restore volume to Sound Bases
      (bind (_keypin_2 _valuepin_2) (Utilities|Map|ForEachLoop(Map) (Variables|SourceAudio|GetSoundBaseMap))
        (:then
          (Class|ReaperAudioHelpers|RestoreSoundBaseVolume _keypin_2 _valuepin_2))))))