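; BP_AudioCapture_Comp captures audio input and visualizes its loudness by scaling a sphere.
; StartAudioCapture and StopAudioCapture control the AudioCaptureInBP component, and EndPlay also stops the capture.
; Each envelope value from the capture is remapped with a clamped range to set the sphere's uniform relative scale, so it grows as the input gets louder.
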(event OnAudioEnvelopeValue(AudioCaptureInBP)
  (params (EnvelopeValue :type Float%20%28single-precision%29))
  (Transformation|SetRelativeScale3D (Variables|Default|GetSphere) (Math|Conversions|ToVector(Float) (Math|Float|MapRangeClamped (+ EnvelopeValue 1.0) 1.0 2.0 1.0 5e+01))))

(event EventEndPlay
  (params (EndPlayReason :type EEndPlayReason%20Enum :default "Destroyed"))
  (Audio|Components|Audio|Stop (Variables|Default|GetAudioCaptureInBP)))

(fn ConstructionScript)

(fn StartAudioCapture
  (CameraShake|Start (Variables|Default|GetAudioCaptureInBP)))

(fn StopAudioCapture
  (Audio|Components|Audio|Stop (Variables|Default|GetAudioCaptureInBP)))